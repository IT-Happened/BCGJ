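; BP_BotCharacter is a bot character Blueprint that handles enemy health display and death.
; OnHealthChanged passes current and max health to the WBP_EnemyHealths widget held by its Widget component.
; OnDeath ragdolls the mesh with physics-only collision, disables capsule collision and destroys the health widget component.
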(fn `On Death`
  (bind _mesh (`self.Mesh`))
  (`PrimitiveComponent.SetCollisionEnabled` _mesh "PhysicsOnly")
  (`PrimitiveComponent.SetSimulatePhysics` _mesh true)
  (`PrimitiveComponent.SetCollisionEnabled` (`self.CapsuleComponent`) "NoCollision")
  (`ActorComponent.K2_DestroyComponent` (`self.Widget`)))

(fn `OnHealthChanged`
  (params (CurrentHealth :type "Float (double-precision)") (MaxHealth :type "Float (double-precision)"))
  (bind _aswbp_enemy_healths (cast `/Game/Game/UI/WBP_EnemyHealths` (`WidgetComponent.GetWidget` (`self.Widget`))))
  (`/Game/Game/UI/WBP_EnemyHealths.SetHealths` _aswbp_enemy_healths CurrentHealth MaxHealth))

(fn `UserConstructionScript`
  (`parent.UserConstructionScript`))