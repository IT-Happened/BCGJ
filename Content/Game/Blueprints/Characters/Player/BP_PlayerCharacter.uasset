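; Player character pawn with axis-driven walking and mouse look, a laser attack, and checkpoint respawn.
; Attack input starts and stops the laser component, while energy and health changes update the HUD, with damage adding an overlay widget and occasional sound on any health change.
; Death shows a widget, then teleports to the stored checkpoint and heals after a short delay.
; Throw-prediction spline helpers exist, but their event-graph calls are disconnected.
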(event `self.ReceiveBeginPlay`
  (`parent.ReceiveBeginPlay`)
  (add `/Game/Game/Blueprints/Components/BP_LaserComponent.EnergyChanged` (`self.BP_LaserComponent`) (`|CreateDelegate` :!event `On Energy Changed`)))

(event `InputAction|Granade`
  (params (Key :type "Key Structure")))

(event `InputAction|Aim`
  (params (Key :type "Key Structure")))

(event `InputAction|Jump`
  (params (Key :type "Key Structure")))

(event `InputAxis|LookRight`
  (params (AxisValue :type "Float (single-precision)"))
  (`self.AddControllerYawInput` AxisValue))

(event `InputAxis|MoveForward`
  (params (AxisValue :type "Float (single-precision)"))
  (bind _output_get (set `self.WalkForward` AxisValue))
  (`self.AddMovementInput` (`self.GetActorForwardVector`) _output_get))

(event `InputAxis|LookUp`
  (params (AxisValue :type "Float (single-precision)"))
  (`self.AddControllerPitchInput` AxisValue))

(event `InputAxis|MoveRight`
  (params (AxisValue :type "Float (single-precision)"))
  (bind _output_get (set `self.WalkRight` AxisValue))
  (`self.AddMovementInput` (`self.GetActorRightVector`) _output_get))

(event `InputAction|Attack`
  (params (Key :type "Key Structure"))
  (:`Pressed`
    (`/Game/Game/Blueprints/Components/BP_LaserComponent.StartUse` (`self.BP_LaserComponent`)))
  (:`Released`
    (`/Game/Game/Blueprints/Components/BP_LaserComponent.StopUse` (`self.BP_LaserComponent`))))

(event `self.On Death`
  (bind _returnvalue (`|CreateWidget` "/Game/Game/UI/WBP_Death.WBP_Death_C"))
  (`UserWidget.AddToViewport` _returnvalue 0)
  (`KismetSystemLibrary.Delay` 0.3)
  (`self.K2_SetActorLocation` (`self.K2_GetActorLocation` (`self.CheckPoint`)) false true)
  (`/Game/Game/Blueprints/Components/BP_HealthComponent.Heal` (`self.BP_HealthComponent`) 10000.0))

(fn `CreatePredictionSpline`
  (bind _returnvalue (`AddComponent|NODE_AddSplineComponent-0`))
  (bind _output_get (set `self.PredictionSpline` _returnvalue))
  (`/Game/Game/Blueprints/Components/BP_ThrowComponent.CreatePredictionSpline` (`self.BP_ThrowComponent`) _output_get))

(fn `CreateSplineMesh`
  (returns (ReturnValue :type "SplineMeshComponent Object Reference"))
  (bind _returnvalue (`AddComponent|NODE_AddSplineMeshComponent-0` :`bManualAttachment` true))
  (return _returnvalue))

(fn `On Energy Changed`
  (params (CurrentEnergy :type "Float (double-precision)") (MaxEnergy :type "Float (double-precision)"))
  (`/Game/Game/UI/BP_HUD.Set Energy` (`/Game/Game/Blueprints/Libraries/BFL_GetInfo.GetHUD`) CurrentEnergy MaxEnergy))

(fn `OnHealthChanged`
  (params (CurrentHealth :type "Float (double-precision)") (MaxHealth :type "Float (double-precision)"))
  (`/Game/Game/UI/BP_HUD.SetHealths` (`/Game/Game/Blueprints/Libraries/BFL_GetInfo.GetHUD`) CurrentHealth MaxHealth)
  (bind _returnvalue (`|CreateWidget` "/Game/Game/UI/WBP_Damage.WBP_Damage_C"))
  (`UserWidget.AddToViewport` _returnvalue 0)
  (if (`KismetMathLibrary.RandomBoolWithWeight` 0.07)
    (`GameplayStatics.PlaySound2D` "/Game/Game/Assets/Sound/Damages/Cue_Damage.Cue_Damage" 1.0 1.0 0.0 null null)))

(fn `SetCheckpoint`
  (params (NewCheckpoint :type "/Game/Game/Blueprints/Checkpoint/BP_CheckPoint Object Reference"))
  (set `self.CheckPoint` NewCheckpoint))

(fn `UserConstructionScript`)