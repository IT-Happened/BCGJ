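; Temporary starting pawn for the scripted intro, with gated look and attack input and no movement.
; Yaw is clamped to an arc, and looking far both left and right plays Seq_Second once.
; An allowed attack shows the scientist attack widget, plays another sequence, then spawns and possesses BP_PlayerCharacter after a short delay, enables HUD rage and destroys this pawn.
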(event `InputAxis|LookRight`
  (params (AxisValue :type "Float (single-precision)"))
  (bind (_returnvalue_roll _returnvalue_pitch _returnvalue_yaw) (`KismetMathLibrary.BreakRotator` (`self.K2_GetActorRotation` (`self.GetController`))))
  (bind _returnvalue (`KismetMathLibrary.FClamp` (+ AxisValue _returnvalue_yaw) 15.0 165.0))
  (if (`self.AllowRotate`)
    (if (< _returnvalue 45.0)
      (set `self.LeftRotate` true)
      (if (== (`self.RightRotate`) (`self.LeftRotate`)) :!label _label
        (`|ExecutionSequence`
          (:`then_0`
            (`/Engine/EditorBlueprintResources/StandardMacros.DoOnce` false
              (:`Completed`
                (bind (_outactor _returnvalue_2) (`LevelSequencePlayer.CreateLevelSequencePlayer` "/Game/Game/Map/Cinematic/Seq_Second.Seq_Second" (make `MovieSceneSequencePlaybackSettings` false (struct) 1.0 0.0 false false true true true true)))
                (`MovieSceneSequencePlayer.Play` _returnvalue_2))))
          (:`then_1`
            (`Controller.SetControlRotation` (`self.GetController`) (`KismetMathLibrary.MakeRotator` _returnvalue_roll _returnvalue_pitch _returnvalue) :!label _label_2)))
        (else
          (goto _label_2)))
      (elif (> _returnvalue 135.0)
        (set `self.RightRotate` true)
        (goto _label)
        (else
          (goto _label_2))))))

(event `InputAxis|MoveForward`
  (params (AxisValue :type "Float (single-precision)")))

(event `InputAxis|MoveRight`
  (params (AxisValue :type "Float (single-precision)")))

(event `InputAxis|LookUp`
  (params (AxisValue :type "Float (single-precision)"))
  (if (`self.AllowRotate`)
    (`self.AddControllerPitchInput` AxisValue)))

(event `InputAction|Attack`
  (params (Key :type "Key Structure"))
  (:`Pressed`
    (if (`self.AllowFire`)
      (`/Game/Game/UI/BP_HUD.StopFirstAttack` (`/Game/Game/Blueprints/Libraries/BFL_GetInfo.GetHUD`))
      (bind _returnvalue (`|CreateWidget` "/Game/Game/UI/WBP_AttackScientist.WBP_AttackScientist_C"))
      (`UserWidget.AddToViewport` _returnvalue 0)
      (bind (_outactor _returnvalue_2) (`LevelSequencePlayer.CreateLevelSequencePlayer` (`self.Seq`)))
      (`MovieSceneSequencePlayer.Play` _returnvalue_2)
      (`KismetSystemLibrary.Delay` 0.2)
      (bind _returnvalue_3 (`|SpawnActorFromClass` "/Game/Game/Blueprints/Characters/Player/BP_PlayerCharacter.BP_PlayerCharacter_C" (`KismetMathLibrary.MakeTransform` (`self.K2_GetActorLocation`) (`self.K2_GetActorRotation`)) "Undefined" "OverrideRootScale" null null))
      (`Controller.Possess` (`GameplayStatics.GetPlayerController` 0) _returnvalue_3)
      (`/Game/Game/UI/BP_HUD.Rage` (`/Game/Game/Blueprints/Libraries/BFL_GetInfo.GetHUD`) true)
      (`self.K2_DestroyActor`))))

(fn `UserConstructionScript`)