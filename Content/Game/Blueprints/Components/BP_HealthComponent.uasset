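; BP_HealthComponent is a component that tracks health for its owning actor.
; On BeginPlay it binds to the owner's OnTakeAnyDamage and subtracts incoming damage from CurrentHealth without clamping.
; Each hit broadcasts HealthChanged with current and max health, then Death whenever health is at or below zero, with no guard against repeat broadcasts.
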(event `self.ReceiveBeginPlay`
  (add `Actor.OnTakeAnyDamage` (`self.GetOwner`) (delegate `OnTakeAnyDamage`)))

(event `OnTakeAnyDamage`
  (params (DamagedActor :type "Actor Object Reference") (Damage :type "Float (double-precision)") (DamageType :type "DamageType Object Reference") (InstigatedBy :type "Controller Object Reference") (DamageCauser :type "Actor Object Reference"))
  (bind _output_get (set `self.CurrentHealth` (- (`self.CurrentHealth`) Damage)))
  (`self.HealthChanged` (`self.CurrentHealth`) (`self.MaxHealth`))
  (if (<= _output_get 0.0)
    (`self.Death`)))