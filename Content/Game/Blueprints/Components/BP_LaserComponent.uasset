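; Laser weapon component that gives its owner a tap-fired beam shot and a hold-activated continuous laser, both powered by shared energy.
; Releasing before the hold timer ends, or lacking the laser upgrade, fires the single beam; holding starts looping laser damage ticks.
; Both modes line-trace from the camera for damage and draw particle beams from the mesh's LaserSocket.
; Spending energy broadcasts changes and restarts delayed timer-based regeneration; depletion stops the laser.
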(fn `Play Laser FX`
  (bind _returnvalue (`GameplayStatics.SpawnEmitterAtLocation` (`self.LaserEmmiterTemplate`)))
  (set `self.LaserParticleRef` _returnvalue)
  (bind _returnvalue_2 (`GameplayStatics.SpawnSound2D` (`self.LaserSound`) 1.0 1.0 0.0 null))
  (bind _output_get (set `self.LaserSoundRef` _returnvalue_2))
  (`AudioComponent.Play` _output_get 0.0))

(fn `RegenerateEnergy`
  (bind _output_get (set `self.CurrentEnergy` (`KismetMathLibrary.FClamp` (+ (* (`self.RegenerateEnergyPerSecond`) (`self.RegenerateEnergyTickTime`)) (`self.CurrentEnergy`)) 0.0 (`self.MaxEnergy`))))
  (`self.EnergyChanged` (`self.CurrentEnergy`) (`self.MaxEnergy`))
  (if (>= _output_get (`self.MaxEnergy`))
    (`self.StopRegenerateEnergy`)))

(fn `StartLaser`
  (`KismetSystemLibrary.K2_SetTimerDelegate` (`|CreateDelegate` :!event `Play Laser FX`) (`self.LaserTickTime`) false 0.1)
  (bind _returnvalue (`KismetSystemLibrary.K2_SetTimerDelegate` (`|CreateDelegate` :!event `Use Tick Laser`) (`self.LaserTickTime`) true 0.1))
  (set `self.LaserTimer` _returnvalue))

(fn `StartRegenerateEnergy`
  (bind _returnvalue (`KismetSystemLibrary.K2_SetTimerDelegate` (`|CreateDelegate` :!event `RegenerateEnergy`) (`self.RegenerateEnergyTickTime`) true (`self.TimeBeforeStartEnergyRegeneration`)))
  (set `self.RegenerationTimer` _returnvalue))

(fn `StartUse`
  (if (`self.CanUse`)
    (if (>= (/ (`self.CurrentEnergy`) (`self.MaxEnergy`)) (`self.MinEnergy % ToUse`))
      (bind _returnvalue (`KismetSystemLibrary.K2_SetTimerDelegate` (`|CreateDelegate` :!event `StartLaser`) (`self.HoldTimeToActivateLaser`)))
      (set `self.StartLaserTimer` _returnvalue)
      (set `self.CanUse` false)
      (if (not (`self.HaveLaser`))
        (`self.StopUse`)))))

(fn `StartUseBeam`
  (`KismetSystemLibrary.K2_SetTimerDelegate` (`|CreateDelegate` :!event `Use Beam`) 0.01))

(fn `StopLaser`
  (`KismetSystemLibrary.K2_ClearAndInvalidateTimerHandle` (`self.LaserTimer`))
  (`KismetSystemLibrary.K2_ClearAndInvalidateTimerHandle` (`self.StartLaserTimer`))
  (`Character.StopAnimMontage` (cast `Character` (`self.GetOwner`) :!pure true) null)
  (`|ExecutionSequence`
    (:`then_0`
      (bind _laserparticleref (`self.LaserParticleRef`)
        (:`then`
          (`self.K2_DestroyComponent` _laserparticleref))
        (:`else`)))
    (:`then_1`
      (bind _lasersoundref (`self.LaserSoundRef`)
        (:`then`
          (`self.K2_DestroyComponent` _lasersoundref))
        (:`else`)))))

(fn `StopRegenerateEnergy`
  (`KismetSystemLibrary.K2_ClearAndInvalidateTimerHandle` (`self.RegenerationTimer`)))

(fn `StopUse`
  (if (`KismetSystemLibrary.K2_TimerExistsHandle` (`self.StartLaserTimer`))
    (`self.StartUseBeam`))
  (set `self.CanUse` true)
  (`self.StopLaser`))

(fn `Use Beam`
  (locals (`_FX EndPoint` :type "Vector Structure" :default (0.0 0.0 0.0)))
  (bind _returnvalue (`Actor.GetComponentByClass` (`self.GetOwner`) "/Script/Engine.CameraComponent"))
  (bind _returnvalue_2 (`SceneComponent.K2_GetComponentLocation` _returnvalue))
  (bind _returnvalue_3 (`SceneComponent.GetForwardVector` _returnvalue))
  (if (>= (`self.CurrentEnergy`) (`self.EnergyToUseBeam`))
    (`self.UseEnergy` (`self.EnergyToUseBeam`))
    (bind (_outhit _returnvalue_4) (`KismetSystemLibrary.LineTraceSingle` (+ (* _returnvalue_3 100.0) _returnvalue_2) (+ _returnvalue_2 (* _returnvalue_3 (`self.BeamRange`))) "TraceTypeQuery4" false (`|MakeArray` (`self.GetOwner`)) "None" true (struct :`R` 1.0 :`A` 1.0) (struct :`G` 1.0 :`A` 1.0) 2.0))
    (if _returnvalue_4
      (bind (_bblockinghit _binitialoverlap _time _distance _location _impactpoint _normal _impactnormal _physmat _hitactor _hitcomponent _hitbonename _hititem _faceindex _tracestart _traceend) (`GameplayStatics.BreakHitResult` _outhit))
      (`GameplayStatics.ApplyDamage` _hitactor (`self.BeamDamage`) null (`self.GetOwner`))
      (set `local._FX EndPoint` _impactpoint)
      (else
        (set `local._FX EndPoint` _traceend)))
    (`GameplayStatics.PlaySound2D` (`self.BeamSound`) 1.0 1.0 0.0 null null)
    (bind _returnvalue_5 (`GameplayStatics.SpawnEmitterAtLocation` (`self.BeamEmmiterTemplate`)))
    (`ParticleSystemComponent.SetBeamSourcePoint` _returnvalue_5 0 (`SceneComponent.GetSocketLocation` (`Actor.GetComponentByClass` (`self.GetOwner`) "/Script/Engine.SkeletalMeshComponent") "LaserSocket") 0)
    (`ParticleSystemComponent.SetBeamEndPoint` _returnvalue_5 0 (`local._FX EndPoint`))))

(fn `Use Tick Laser`
  (locals (_NeedEnergy :type "Float (double-precision)") (`_FX EndPoint` :type "Vector Structure"))
  (bind _returnvalue (`Actor.GetComponentByClass` (`self.GetOwner`) "/Script/Engine.CameraComponent"))
  (bind _returnvalue_2 (`SceneComponent.GetSocketLocation` (`Actor.GetComponentByClass` (`self.GetOwner`) "/Script/Engine.SkeletalMeshComponent") "LaserSocket"))
  (bind _returnvalue_3 (`SceneComponent.K2_GetComponentLocation` _returnvalue))
  (set `local._NeedEnergy` (* (`self.EnergyPerSecondToUseLaser`) (`self.LaserTickTime`)))
  (if (>= (`self.CurrentEnergy`) (`local._NeedEnergy`))
    (`self.UseEnergy` (`local._NeedEnergy`))
    (bind (_outhit _returnvalue_4) (`KismetSystemLibrary.LineTraceSingle` _returnvalue_3 (+ _returnvalue_3 (* (`SceneComponent.GetForwardVector` _returnvalue) (`self.LaserRange`))) "TraceTypeQuery4" false (`|MakeArray` (`self.GetOwner`))))
    (if _returnvalue_4
      (bind (_bblockinghit _binitialoverlap _time _distance _location _impactpoint _normal _impactnormal _physmat _hitactor _hitcomponent _hitbonename _hititem _faceindex _tracestart _traceend) (`GameplayStatics.BreakHitResult` _outhit))
      (`GameplayStatics.ApplyDamage` _hitactor (* (`self.DamagePerSecond`) (`self.LaserTickTime`)) null (`self.GetOwner`) "/Game/Game/Blueprints/Weapons/DT_Laser.DT_Laser_C")
      (set `local._FX EndPoint` _impactpoint)
      (else
        (set `local._FX EndPoint` _traceend)))
    (bind _laserparticleref (`self.LaserParticleRef`)
      (:`then`
        (`ParticleSystemComponent.SetBeamSourcePoint` _laserparticleref 1 _returnvalue_2 0)
        (`ParticleSystemComponent.SetBeamTargetPoint` _laserparticleref 1 (`local._FX EndPoint`) 0)
        (`ParticleSystemComponent.SetBeamSourcePoint` _laserparticleref 0 _returnvalue_2 0)
        (`ParticleSystemComponent.SetBeamTargetPoint` _laserparticleref 0 (`local._FX EndPoint`) 0))
      (:`else`))))

(fn `UseEnergy`
  (params (Energy :type "Float (double-precision)"))
  (bind _output_get (set `self.CurrentEnergy` (- (`self.CurrentEnergy`) Energy)))
  (`self.EnergyChanged` (`self.CurrentEnergy`) (`self.MaxEnergy`))
  (`self.StopRegenerateEnergy`)
  (if (<= _output_get 0.0)
    (`self.StopLaser`))
  (`self.StartRegenerateEnergy`))