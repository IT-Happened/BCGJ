(event `self.ReceiveTick`
  (params (DeltaSeconds :type "Float (single-precision)"))
  (`self.DrawPredictionSpline`))

(fn `CreatePredictionSpline`
  (params (PredictionSpline :type "SplineComponent Object Reference"))
  (set `self.PredictionSpline` PredictionSpline)
  (bind _returnvalue (`|SpawnActorFromClass` "/Game/Game/Blueprints/Weapons/BP_PredictionEndPoint.BP_PredictionEndPoint_C" (`KismetMathLibrary.MakeTransform` (0.0 0.0 0.0)) "Undefined" "OverrideRootScale" null null))
  (bind _output_get (set `self.PredictionEndPoint` _returnvalue))
  (`Actor.SetActorHiddenInGame` _output_get false))

(fn `DestroyPredictionMeshes`
  (for _array_element (`self.PredictionSplineMeshes`)
    (`self.K2_DestroyComponent` _array_element))
  (`KismetArrayLibrary.Array_Clear` (`self.PredictionSplineMeshes`)))

(fn `DestroyPredictionSpline`
  (bind _predictionspline (`self.PredictionSpline`)
    (:`then`
      (`self.K2_DestroyComponent` _predictionspline)
      (set `self.PredictionSpline` null))
    (:`else`
      _))
  (`self.DestroyPredictionMeshes`)
  (`Actor.K2_DestroyActor` (`self.PredictionEndPoint`))
  (set `self.PredictionEndPoint` null))

(fn `DrawPredictionSpline`
  (bind _predictionendpoint (`self.PredictionEndPoint`))
  (`self.PredictionSplineValid`
    (:`Is Valid`
      (`|ExecutionSequence`
        (:`then_0`
          (bind (_outhit _outpathpositions _outlasttracedestination _returnvalue) (`GameplayStatics.Blueprint_PredictProjectilePath_ByTraceChannel` (`self.ThrowLocation`) (`self.ThrowVelocity`) true 25.0 "ECC_WorldDynamic" false (`|MakeArray` (`self.GetOwner`))))
          (if _returnvalue
            (`Actor.SetActorHiddenInGame` _predictionendpoint false)
            (`Actor.K2_SetActorLocation` _predictionendpoint (`.ImpactPoint` (`GameplayStatics.BreakHitResult` _outhit)) false true)
            (else
              (`Actor.SetActorHiddenInGame` (`self.PredictionEndPoint`) true)))
          (`SplineComponent.SetSplinePoints` (`self.PredictionSpline`) _outpathpositions "World" true)
          (`self.DestroyPredictionMeshes`))
        (:`then_1`
          (for _index (range (+ (`KismetMathLibrary.FTrunc` (/ (`SplineComponent.GetSplineLength` (`self.PredictionSpline`)) 100.0)) 1))
            (set `self.Index` _index)
            (bind _asbp_player_character (cast `/Game/Game/Blueprints/Characters/Player/BP_PlayerCharacter` (`self.GetOwner`)))
            (bind _returnvalue_2 (`/Game/Game/Blueprints/Characters/Player/BP_PlayerCharacter.CreateSplineMesh` _asbp_player_character))
            (`KismetArrayLibrary.Array_Add` (`self.PredictionSplineMeshes`) _returnvalue_2)
            (`SplineMeshComponent.SetStartAndEnd` _returnvalue_2 (`SplineComponent.GetLocationAtDistanceAlongSpline` (`self.PredictionSpline`) (* (`self.Index`) 100.0) "World") (0.0 0.0 0.0) (`SplineComponent.GetLocationAtDistanceAlongSpline` (`self.PredictionSpline`) (* (+ (`self.Index`) 1) 100.0) "World") (0.0 0.0 0.0) true)))))))