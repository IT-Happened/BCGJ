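; Base weapon Blueprint that supplies fire-rate gating, with an empty Shoot function as the slot for actual firing behavior.
; StartFire acts only while IsCanShoot is true: it clears the flag, calls Shoot and starts a one-shot timer of 60 / FireRate seconds, treating FireRate as rounds per minute.
; EndFire sets IsCanShoot back to true, and the event graph has no active logic.
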(fn `EndFire`
  (set `self.IsCanShoot` true))

(fn `Shoot`)

(fn `StartFire`
  (if (`self.IsCanShoot`)
    (set `self.IsCanShoot` false)
    (`self.Shoot`)
    (`KismetSystemLibrary.K2_SetTimerDelegate` (`|CreateDelegate` :!event `EndFire`) (/ 60.0 (`self.FireRate`)))
    (else
      (return))))

(fn `UserConstructionScript`)