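; BP_Rifle is a hitscan rifle weapon whose shots damage only the player character.
; Shoot plays the fire animation on the skeletal mesh and line traces from the owner's eye point out to ShootingRange.
; The trace direction is randomized within a cone around the owning controller's forward vector to create spread.
; A hit on BP_PlayerCharacter applies Damage, crediting the owner's controller as instigator.
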(fn `Shoot`
  (bind _returnvalue (`self.GetOwner`))
  (bind _returnvalue_2 (`self.GetOwner`))
  (bind _outlocation (`self.GetActorEyesViewPoint` _returnvalue))
  (`SkeletalMeshComponent.PlayAnimation` (`self.SkeletalMesh`) "/Game/MilitaryWeapSilver/Weapons/Animations/Fire_Rifle_W.Fire_Rifle_W" false)
  (bind (_outhit _returnvalue_3) (`KismetSystemLibrary.LineTraceSingle` _outlocation (+ _outlocation (* (`KismetMathLibrary.RandomUnitVectorInConeInRadians` (`self.GetActorForwardVector` (`Pawn.GetController` (cast `Pawn` _returnvalue :!pure true))) 0.2) (`self.Shooting Range`))) "TraceTypeQuery4" false (`|MakeArray` _returnvalue) "None" true (struct :`R` 1.0 :`A` 1.0) (struct :`G` 1.0 :`A` 1.0) 1.0))
  (if _returnvalue_3
    (bind _asbp_player_character (cast `/Game/Game/Blueprints/Characters/Player/BP_PlayerCharacter` (`.HitActor` (`GameplayStatics.BreakHitResult` _outhit))))
    (`GameplayStatics.ApplyDamage` _asbp_player_character (`self.Damage`) (`Pawn.GetController` (cast `Pawn` _returnvalue_2 :!pure true)) _returnvalue_2)))

(fn `UserConstructionScript`
  (`parent.UserConstructionScript`))